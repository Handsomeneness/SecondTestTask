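; BP_SoccerGoal is a soccer goal actor that detects a ball entering it and respawns a new one.
; On BeginPlay it caches the location of the referenced ball as the spawn point.
; When a BP_SoccerBall overlaps the Box, it plays a hit particle above the goal and destroys the ball.
; After a two-second delay it spawns a fresh ball at the cached location.
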(event OnComponentBeginOverlap(Box)
  (params (OverlappedComponent :type Primitive%20Component%20Object%20Reference) (OtherActor :type Actor%20Object%20Reference) (OtherComp :type Primitive%20Component%20Object%20Reference) (OtherBodyIndex :type Integer) (bFromSweep :type Boolean) (SweepResult :type Hit%20Result%20Structure%20%28by%20ref%29))
  (bind _soccergoal (Variables|Default|GetSoccerGoal))
  (bind _returnvalue (Transformation|GetWorldLocation _soccergoal))
  (bind (_x _y) (Math|Vector|BreakVector _returnvalue))
  (bind _asbp_soccer_ball (Utilities|Casting|CastToBP_SoccerBall OtherActor))
  (Effects|SpawnEmitteratLocation "/Game/FXVarietyPack/Particles/P_ky_hit2.P_ky_hit2" (Math|Vector|MakeVector _x _y 3e+02))
  (Actor|DestroyActor _asbp_soccer_ball)
  (Utilities|FlowControl|Delay 2.0)
  (Game|SpawnActorfromClass "/Game/Blueprints/SoccerBlueprints/BP_SoccerBall.BP_SoccerBall_C" (Math|Transform|MakeTransform (Variables|Default|GetBallSpawnLocation) "0, 0, 0" "1.000000,1.000000,1.000000") "Undefined" 0 0))

(event EventBeginPlay
  (bind _soccerballref (Variables|Default|GetSoccerBallRef))
  (Utilities|IsValid _soccerballref
    (:Is%20Valid
      (Variables|Default|SetBallSpawnLocation (Transformation|GetActorLocation _soccerballref)))))

(fn ConstructionScript)