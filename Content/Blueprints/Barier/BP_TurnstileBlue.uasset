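; BP_TurnstileBlue is a turnstile barrier that opens for a player holding a blue ticket.
; Its interaction collision caches the overlapping third-person character and toggles player 0 input on entry and exit.
; Two separate E-key handlers each identify the selected item by icon, consume it via UseItem and play a timeline rotating the left or right border's yaw.
; Only the left-border handler prints Russian success or wrong-ticket messages.
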(event OnComponentBeginOverlap(InterractCollision)
  (params (OverlappedComponent :type Primitive%20Component%20Object%20Reference) (OtherActor :type Actor%20Object%20Reference) (OtherComp :type Primitive%20Component%20Object%20Reference) (OtherBodyIndex :type Integer) (bFromSweep :type Boolean) (SweepResult :type Hit%20Result%20Structure%20%28by%20ref%29))
  (bind _asbp_third_person_character (Utilities|Casting|CastToBP_ThirdPersonCharacter OtherActor))
  (Input|EnableInput (Game|GetPlayerController 0)))

(event OnComponentEndOverlap(InterractCollision)
  (params (OverlappedComponent :type Primitive%20Component%20Object%20Reference) (OtherActor :type Actor%20Object%20Reference) (OtherComp :type Primitive%20Component%20Object%20Reference) (OtherBodyIndex :type Integer))
  (Utilities|Casting|CastToBP_ThirdPersonCharacter OtherActor)
  (Input|DisableInput (Game|GetPlayerController 0)))

(event Input|KeyboardEvents|E
  (params (Key :type Key%20Structure :default "None"))
  (:Pressed
    (if (== (.ItemIcon (Utilities|Struct|BreakItemStruct (Utilities|Array|Get(acopy) (Variables|/Game/ThirdPerson/Blueprints/BP_ThirdPersonCharacter.BP_ThirdPersonCharacter_C|GetInventoryArray (stale OnComponentBeginOverlap(InterractCollision) _asbp_third_person_character)) (Variables|/Game/ThirdPerson/Blueprints/BP_ThirdPersonCharacter.BP_ThirdPersonCharacter_C|GetSelectedIndex (stale OnComponentBeginOverlap(InterractCollision) _asbp_third_person_character))))) "/Game/Blueprints/Barier/ticket-low-poly/source/BlueTicket.BlueTicket")
      (Development|PrintString "ИСПОЛЬЗОВАН СИНИЙ БИЛЕТ" true true "(R=0.030354,G=0.364353,B=1.000000,A=1.000000)" 3.0)
      (Default|UseItem (stale OnComponentBeginOverlap(InterractCollision) _asbp_third_person_character) (Utilities|Array|Get(acopy) (Variables|/Game/ThirdPerson/Blueprints/BP_ThirdPersonCharacter.BP_ThirdPersonCharacter_C|GetInventoryArray (stale OnComponentBeginOverlap(InterractCollision) _asbp_third_person_character)) (Variables|/Game/ThirdPerson/Blueprints/BP_ThirdPersonCharacter.BP_ThirdPersonCharacter_C|GetSelectedIndex (stale OnComponentBeginOverlap(InterractCollision) _asbp_third_person_character))))
      (bind _newtrack_0 (Timeline|Timeline Play)
        (:Update
          (Transformation|SetRelativeRotation (Variables|Default|GetLeftBorder) (Math|Rotator|MakeRotator 0.0 0.0 _newtrack_0) false false)))
      (else
        (Development|PrintString "ИСПОЛЬЗОВАН НЕВЕРНЫЙ БИЛЕТ" true true "(R=0.000000,G=0.361448,B=1.000000,A=1.000000)" 3.0)))))

(event Input|KeyboardEvents|E
  (params (Key :type Key%20Structure :default "None"))
  (:Pressed
    (if (== (.ItemIcon (Utilities|Struct|BreakItemStruct (Utilities|Array|Get(acopy) (Variables|/Game/ThirdPerson/Blueprints/BP_ThirdPersonCharacter.BP_ThirdPersonCharacter_C|GetInventoryArray (stale OnComponentBeginOverlap(InterractCollision) _asbp_third_person_character)) (Variables|/Game/ThirdPerson/Blueprints/BP_ThirdPersonCharacter.BP_ThirdPersonCharacter_C|GetSelectedIndex (stale OnComponentBeginOverlap(InterractCollision) _asbp_third_person_character))))) "/Game/Blueprints/Barier/ticket-low-poly/source/BlueTicket.BlueTicket")
      (Default|UseItem (stale OnComponentBeginOverlap(InterractCollision) _asbp_third_person_character) (Utilities|Array|Get(acopy) (Variables|/Game/ThirdPerson/Blueprints/BP_ThirdPersonCharacter.BP_ThirdPersonCharacter_C|GetInventoryArray (stale OnComponentBeginOverlap(InterractCollision) _asbp_third_person_character)) (Variables|/Game/ThirdPerson/Blueprints/BP_ThirdPersonCharacter.BP_ThirdPersonCharacter_C|GetSelectedIndex (stale OnComponentBeginOverlap(InterractCollision) _asbp_third_person_character))))
      (bind _newtrack_0 (Timeline|Timeline_0 Play)
        (:Update
          (Transformation|SetRelativeRotation (Variables|Default|GetRightBorder) (Math|Rotator|MakeRotator 0.0 0.0 _newtrack_0) false false))))))

(fn ConstructionScript)